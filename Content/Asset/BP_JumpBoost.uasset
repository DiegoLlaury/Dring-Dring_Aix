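; BP_JumpBoost is a jump boost pickup that a BP_Phone actor collects on overlapping its sphere.
; If the phone's DoubleJump flag is not already set, it spawns two effects at its location and calls JumpBoostMessage on the phone with that location.
; It then destroys itself after a short delay, leaving any change to the jump state to BP_Phone.
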(event `self.Sphere.OnComponentBeginOverlap`
  (params (OverlappedComponent :type "PrimitiveComponent Object Reference") (OtherActor :type "Actor Object Reference") (OtherComp :type "PrimitiveComponent Object Reference") (OtherBodyIndex :type Integer) (bFromSweep :type Boolean) (SweepResult :type "HitResult Structure (by ref)"))
  (bind _returnvalue (`self.K2_GetActorLocation` self))
  (bind _asbp_phone (cast `/Game/Phone/BP/BP_Phone` OtherActor))
  (if (not (`/Game/Phone/BP/BP_Phone.DoubleJump` _asbp_phone))
    (`NiagaraFunctionLibrary.SpawnSystemAtLocation` "/Game/Asset/EnergyExplosion.EnergyExplosion" (`self.K2_GetActorLocation` self))
    (`NiagaraFunctionLibrary.SpawnSystemAtLocation` "/Game/Asset/NS_pilecburst.NS_pilecburst" _returnvalue)
    (message `/Game/Asset/BPI_doublejump.JumpBoost` _asbp_phone _returnvalue)
    (`KismetSystemLibrary.Delay` 0.2)
    (`self.K2_DestroyActor`)))

(fn `UserConstructionScript`)