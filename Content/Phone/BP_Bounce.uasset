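; BP_Bounce is a bag-of-chips actor that gives BP_Phone a stronger bounce when the two collide.
; On a hit to the chips component, it looks up BP_Phone with GetActorOfClass and checks that it is the other actor.
; It temporarily doubles the phone's BounceC, calls BounceChips on the phone, then restores the saved value.
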(event `self.bagofchips1.OnComponentHit`
  (params (HitComponent :type "PrimitiveComponent Object Reference") (OtherActor :type "Actor Object Reference") (OtherComp :type "PrimitiveComponent Object Reference") (NormalImpulse :type "Vector Structure") (Hit :type "HitResult Structure (by ref)"))
  (bind _bp_phone (`self.BP_Phone`))
  (bind _bouncec (`/Game/Phone/BP/BP_Phone.BounceC` _bp_phone))
  (bind _returnvalue (`GameplayStatics.GetActorOfClass` "/Game/Phone/BP/BP_Phone.BP_Phone_C"))
  (set `self.BP_Phone` _returnvalue)
  (if (== _returnvalue OtherActor)
    (set `self.BounceFloat` _bouncec)
    (set `/Game/Phone/BP/BP_Phone.BounceC` (* _bouncec 2.0) _bp_phone)
    (`/Game/Phone/BP/BP_Phone.BounceChips` _bp_phone)
    (set `/Game/Phone/BP/BP_Phone.BounceC` (`self.BounceFloat`) _bp_phone)))

(fn `UserConstructionScript`)