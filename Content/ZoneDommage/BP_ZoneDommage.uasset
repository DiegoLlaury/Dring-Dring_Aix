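; BP_ZoneDommage is a damage zone that hurts BP_Phone while it is inside its Box trigger.
; Begin overlap sets InZone and starts a looping one-second timer that applies fixed damage, plays a sound and spawns an explosion effect at the phone.
; End overlap only clears InZone, so the timer stops itself after its next tick, which still deals damage.
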(event `ApplyDamage`
  (`GameplayStatics.ApplyDamage` (stale `self.Box.OnComponentBeginOverlap` _asbp_phone) 8.0)
  (bind _returnvalue (`GameplayStatics.GetActorOfClass` "/Game/Phone/BP/BP_Phone.BP_Phone_C"))
  (bind _asbp_phone (cast `/Game/Phone/BP/BP_Phone` _returnvalue))
  (`GameplayStatics.PlaySound2D` "/Game/SoundDesign/SC_Damage.SC_Damage" 1.0 1.0 0.0 null null)
  (`NiagaraFunctionLibrary.SpawnSystemAtLocation` "/Game/Asset/EnergyExplosion.EnergyExplosion" (`self.K2_GetActorLocation` _asbp_phone))
  (if (not (`self.InZone`))
    (`KismetSystemLibrary.K2_ClearAndInvalidateTimerHandle` (stale `self.Box.OnComponentBeginOverlap` _returnvalue))))

(event `self.Box.OnComponentBeginOverlap`
  (params (OverlappedComponent :type "PrimitiveComponent Object Reference") (OtherActor :type "Actor Object Reference") (OtherComp :type "PrimitiveComponent Object Reference") (OtherBodyIndex :type Integer) (bFromSweep :type Boolean) (SweepResult :type "HitResult Structure (by ref)"))
  (bind _asbp_phone (cast `/Game/Phone/BP/BP_Phone` OtherActor))
  (`/Engine/EditorBlueprintResources/StandardMacros.IsValid` _asbp_phone
    (:`Is Valid`
      (set `self.InZone` true)
      (if (`self.InZone`)
        (bind _returnvalue (`KismetSystemLibrary.K2_SetTimerDelegate` (delegate `ApplyDamage`) 1.0 true))))
    (:`Is Not Valid`
      (set `self.InZone` false))))

(event `self.Box.OnComponentEndOverlap`
  (params (OverlappedComponent :type "PrimitiveComponent Object Reference") (OtherActor :type "Actor Object Reference") (OtherComp :type "PrimitiveComponent Object Reference") (OtherBodyIndex :type Integer))
  (cast `/Game/Phone/BP/BP_Phone` OtherActor)
  (set `self.InZone` false))

(fn `UserConstructionScript`)